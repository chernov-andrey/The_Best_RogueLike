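; NewGameInstance is a game instance Blueprint that shows the main menu, option and pause UI screens.
; Each show event creates its widget on first use, caches it in a variable and adds it to the viewport on every call.
; The main menu widget also has its ModMenu set to "first" when it is first created.
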(event Custom|Show_Main_menu
  (Utilities|IsValid (Variables|Default|GetMain_Menu_WD)
    (:Is%20Valid
      _)
    (:Is%20Not%20Valid
      (bind _returnvalue (UserInterface|CreateWidget "/Game/UMG/WD_MainMenu.WD_MainMenu_C"))
      (bind _output_get (Variables|Default|SetMain_Menu_WD _returnvalue))
      (Variables|/Game/UMG/WD_MainMenu.WD_MainMenu_C|SetMod_Menu _output_get "first")))
  (UserInterface|Viewport|AddtoViewport _output_get 0))

(event Custom|Show_Option
  (Utilities|IsValid (Variables|Default|GetOption_WD)
    (:Is%20Valid
      _)
    (:Is%20Not%20Valid
      (bind _returnvalue (UserInterface|CreateWidget "/Game/UMG/WD_Option.WD_Option_C"))
      (bind _output_get (Variables|Default|SetOption_WD _returnvalue))))
  (UserInterface|Viewport|AddtoViewport _output_get 0))

(event Custom|Show_Pause
  (Utilities|IsValid (Variables|Default|GetPause_WD)
    (:Is%20Valid
      _)
    (:Is%20Not%20Valid
      (bind _returnvalue (UserInterface|CreateWidget "/Game/UMG/WD_Game_Pause.WD_Game_Pause_C"))
      (bind _output_get (Variables|Default|SetPause_WD _returnvalue))))
  (UserInterface|Viewport|AddtoViewport _output_get 0))