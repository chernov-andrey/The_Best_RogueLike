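; Procedural dungeon constructor Blueprint that currently generates the floor of one randomly sized rectangular room.
; The Construction Script rolls a width and height, then nested loops add static mesh components as floor tiles on a fixed-spacing grid from the local origin.
; The room loop runs only once, as the random room-count calculation is left unconnected, and the event graph is empty.
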(event EventBeginPlay)

(event Collision|EventActorBeginOverlap
  (params (OtherActor :type Actor%20Object%20Reference)))

(event EventTick
  (params (DeltaSeconds :type Float%20%28single-precision%29)))

(fn ConstructionScript
  (Variables|Default|SetPosition_Make_floor (Math|Transform|MakeTransform "0, 0, 0"))
  ;[1 1 1] Определяем сколько будет комнат
  (for _index (range 0 0)
    ;[1 1 1] Определяем форму комнаты
    (bind _output_get (Variables|Default|SetWeigt_room (Math|Random|RandomIntegerinRange 2 5)))
    (bind _output_get_2 (Variables|Default|SetHeight_room (Math|Random|RandomIntegerinRange 2 5)))
    (for _index_2 (range 0 _output_get)
      (for _index_3 (range 0 _output_get_2)
        ;;[1 1 1] Cоздаем пол
        (AddComponent|AddStaticMeshComponent false (Math|Transform|MakeTransform (Math|Vector|MakeVector (+ (* _index_2 2e+02) (.X (Math|Vector|BreakVector (.Location (Math|Transform|BreakTransform (Variables|Default|GetPosition_Make_floor)))))) (+ (* _index_3 2e+02) (.Y (Math|Vector|BreakVector (.Location (Math|Transform|BreakTransform (Variables|Default|GetPosition_Make_floor)))))) (.Z (Math|Vector|BreakVector (.Location (Math|Transform|BreakTransform (Variables|Default|GetPosition_Make_floor)))))) (.Rotation (Math|Transform|BreakTransform (Variables|Default|GetPosition_Make_floor))) (.Scale (Math|Transform|BreakTransform (Variables|Default|GetPosition_Make_floor)))))))))