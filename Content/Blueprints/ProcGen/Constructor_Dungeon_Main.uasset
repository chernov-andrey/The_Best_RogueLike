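; Procedural dungeon generator that, on BeginPlay, grows a layout of Constructor_Dungeon rooms until no open doors remain.
; SpawnRoom gives each room a weighted random door count and a shuffled side order that favours opposite doors, then queues its doors.
; AlignRoomDoor rotates the room onto the oldest open door, then uses box overlaps to step it outward while blocked, raising hit meshes and printing debug output.
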(event EventBeginPlay
  (bind _stack_void_doors (Variables|Default|GetStack_Void_Doors))
  (CallFunction|SpawnRoom (Variables|Default|GetStack_Void_Doors) (Variables|Default|GetList_Room) (Variables|Default|GetOrder_Direction) 0 1 (Utilities|Array|MakeArray 1 0 0 0) true)
  (Variables|Default|SetCount_Room 1)
  (while (> (Utilities|Array|Length (Variables|Default|GetStack_Void_Doors)) 0)
    (bind (_first_door _new_room) (CallFunction|SpawnRoom (Variables|Default|GetStack_Void_Doors) (Variables|Default|GetList_Room) (Variables|Default|GetOrder_Direction) 1 2 (Utilities|Array|MakeArray 2 2 1 1) false))
    (CallFunction|AlignRoomDoor (Utilities|Array|Get(acopy) _stack_void_doors) _first_door _new_room _stack_void_doors)
    (Math|Integer|IncrementInt (Variables|Default|GetCount_Room))))

(fn ConstructionScript)

(fn Random4inChance
  (params (Chance_1 :type Integer) (Chance_2 :type Integer) (Chance_3 :type Integer) (Chance_4 :type Integer))
  (bind _output_get (LocalVariables|SetRandom_int (Math|Random|RandomIntegerinRange 0 (+ Chance_1 Chance_2 Chance_3 Chance_4))))
  (if (<= _output_get Chance_1)
    (return 1)
    (elif (<= _output_get (+ Chance_1 Chance_2))
      (return 2)
      (elif true
        (return 3)
        (elif true
          (return 4))))))

(fn MixArray
  (params (Order_dir_dor :type Array%20of%20Strings) (Chance_Straight :type Integer) (Chance_Turn :type Integer))
  (bind _returnvalue (Math|Random|RandomBool))
  (bind _returnvalue_2 (Math|Random|RandomBool))
  (bind _returnvalue_3 (Utilities|String|MakeLiteralString "Top"))
  (bind _returnvalue_4 (Utilities|String|MakeLiteralString "Right"))
  (bind _returnvalue_5 (Utilities|String|MakeLiteralString "Left"))
  (bind _returnvalue_6 (Utilities|String|MakeLiteralString "Dawn"))
  (bind _output (Utilities|Array|Get(acopy) Order_dir_dor))
  (bind _output_2 (Utilities|Array|Get(acopy) Order_dir_dor))
  (bind _returnvalue_7 (select _returnvalue _returnvalue_3 _returnvalue_6))
  (bind _returnvalue_8 (select _returnvalue_2 _returnvalue_4 _returnvalue_5))
  (Utilities|Array|SetArrayElem Order_dir_dor 0 (Utilities|Array|Get(acopy) (LocalVariables|GetStack_direct) (Math|Random|RandomIntegerinRange 0 3)))
  (Utilities|Array|RemoveItem (LocalVariables|GetStack_direct) (Utilities|Array|Get(acopy) Order_dir_dor))
  (if (>= Chance_Straight (Math|Random|RandomIntegerinRange 0 (+ Chance_Straight Chance_Turn)))
    (if (== _output_2 "Dawn")
      (Utilities|Array|SetArrayElem Order_dir_dor 1 "Top")
      (Utilities|Array|RemoveItem (LocalVariables|GetStack_direct) (Utilities|Array|Get(acopy) Order_dir_dor 1) :!label _label)
      (Utilities|Array|SetArrayElem Order_dir_dor 2 (Utilities|Array|Get(acopy) (LocalVariables|GetStack_direct) (Math|Random|RandomIntegerinRange 0 1)) :!label _label_2)
      (Utilities|Array|RemoveItem (LocalVariables|GetStack_direct) (Utilities|Array|Get(acopy) Order_dir_dor 2))
      (Utilities|Array|SetArrayElem Order_dir_dor 3 (Utilities|Array|Get(acopy) (LocalVariables|GetStack_direct)))
      (return)
      (elif (== _output_2 "Left")
        (Utilities|Array|SetArrayElem Order_dir_dor 1 "Right")
        (goto _label)
        (elif (== _output_2 "Top")
          (Utilities|Array|SetArrayElem Order_dir_dor 1 "Dawn")
          (goto _label)
          (elif (== _output_2 "Right")
            (Utilities|Array|SetArrayElem Order_dir_dor 1 "Left")
            (goto _label)
            (else
              (Development|PrintString "Ошибка, непредвиденое значение" true true "(R=0.630208,G=0.000000,B=0.059981,A=1.000000)" 15.0))))))
    (elif (== _output "Dawn")
      (Utilities|Array|SetArrayElem Order_dir_dor 1 _returnvalue_8)
      (Utilities|Array|RemoveItem (LocalVariables|GetStack_direct) (Utilities|Array|Get(acopy) Order_dir_dor 1) :!label _label_3)
      (goto _label_2)
      (elif (== _output "Left")
        (Utilities|Array|SetArrayElem Order_dir_dor 1 _returnvalue_7)
        (goto _label_3)
        (elif (== _output "Top")
          (Utilities|Array|SetArrayElem Order_dir_dor 1 _returnvalue_8)
          (goto _label_3)
          (elif (== _output "Right")
            (Utilities|Array|SetArrayElem Order_dir_dor 1 _returnvalue_7)
            (goto _label_3)))))))

(fn FillLocationMap
  (params (Count_door :type Integer) (Order_Dir :type Array%20of%20Strings))
  (LocalVariables|SetMapLocDoor (Utilities|Map|MakeMap))
  (for _array_element Order_Dir
    (if (> Count_door 0)
      (Utilities|Map|Add (LocalVariables|GetMapLocDoor) _array_element true)
      (Math|Integer|DecrementInt Count_door)
      (else
        (Utilities|Map|Add (LocalVariables|GetMapLocDoor) _array_element false))))
  (return (LocalVariables|GetMapLocDoor)))

(fn SpawnRoom
  (params (Array_door :type Array%20of%20Static%20Mesh%20Component%20Object%20References) (Lisr_room :type Array%20of%20Constructor%20Dungeon%20Object%20References) (Order_Dir :type Array%20of%20Strings) (i :type Integer) (Count_Door :type Integer) (Cout_Door_Chance :type Array%20of%20Integers) (Dont_turn :type Boolean))
  (CallFunction|MixArray Order_Dir 2 1)
  (bind _count_door (CallFunction|Random4inChance (Utilities|Array|Get(acopy) Cout_Door_Chance) (Utilities|Array|Get(acopy) Cout_Door_Chance 1) (Utilities|Array|Get(acopy) Cout_Door_Chance 2) (Utilities|Array|Get(acopy) Cout_Door_Chance 3)))
  (bind _map_loc_door (CallFunction|FillLocationMap _count_door Order_Dir))
  (bind _returnvalue (Game|SpawnActorfromClass "/Game/Blueprints/ProcGen/Constructor_Dungeon.Constructor_Dungeon_C" (Math|Transform|MakeTransform "0, 0, 0" "0, 0, 0" "1,1,1") "Undefined" 0 _map_loc_door (Utilities|Select :Index i :Option%200 "/Game/Blueprints/ProcGen/WallBlock_2.WallBlock_2" :Option%201 "/Game/Blueprints/ProcGen/WallBlock.WallBlock") Dont_turn 0))
  (Utilities|Array|Add (Variables|Default|GetList_Room) _returnvalue)
  (for _array_element (Variables|/Game/Blueprints/ProcGen/Constructor_Dungeon.Constructor_Dungeon_C|GetDoors_in_Room _returnvalue)
    (Utilities|Array|Add Array_door _array_element))
  (return (Utilities|Array|Get(acopy) (Variables|/Game/Blueprints/ProcGen/Constructor_Dungeon.Constructor_Dungeon_C|GetDoors_in_Room _returnvalue)) _returnvalue))

(fn AlignRoomDoor
  (params (Door_in :type Static%20Mesh%20Component%20Object%20Reference) (Door_out :type Static%20Mesh%20Component%20Object%20Reference) (New_Room :type Constructor%20Dungeon%20Object%20Reference) (Array_for_delete :type Array%20of%20Static%20Mesh%20Component%20Object%20References))
  (bind _returnvalue (Transformation|GetActorTransform New_Room))
  (bind _returnvalue_2 (Transformation|GetWorldTransform Door_in))
  (bind _returnvalue_3 (Transformation|GetWorldTransform Door_out))
  (bind _size_box_room (Variables|/Game/Blueprints/ProcGen/Constructor_Dungeon.Constructor_Dungeon_C|GetSize_Box_Room New_Room))
  (bind (_location _rotation) (Math|Transform|BreakTransform _returnvalue_3))
  (bind (_location_2 _rotation_2) (Math|Transform|BreakTransform _returnvalue_2))
  (bind _output_get (LocalVariables|SetChange_angle (- (+ (.yaw _rotation_2) 1.8e+02) (.yaw _rotation))))
  (bind _output_get_2 (LocalVariables|SetChanges_location (- _location_2 (Math|Vector|RotateVectorAroundAxis _location (LocalVariables|GetChange_angle) "0, 0,1.000000"))))
  (bind _output_get_3 (LocalVariables|SetDirection_Step_Change_location (* (Math|Vector|MakeVector (Math|Trig|Sin(Degrees) (.yaw _rotation_2)) (* (Math|Trig|Cos(Degrees) (.yaw _rotation_2)) -1.0) 0.0) (Variables|/Game/Blueprints/ProcGen/Constructor_Dungeon.Constructor_Dungeon_C|GetScale_Index New_Room))))
  (Transformation|SetActorTransform New_Room (Math|Transform|MakeTransform (+ _output_get_2 _output_get_3) (Math|Rotator|MakeRotator 0.0 0.0 _output_get) "1,1,1"))
  (for (_array_element _array_index) _size_box_room
    (Utilities|Array|SetArrayElem _size_box_room _array_index (Math|Transform|MakeTransform (+ (LocalVariables|GetChanges_location) (Math|Vector|RotateVectorAroundAxis (.Location (Math|Transform|BreakTransform _array_element)) (LocalVariables|GetChange_angle) "0, 0,1.000000") (LocalVariables|GetDirection_Step_Change_location)) (.Rotation (Math|Transform|BreakTransform _array_element)) (Math|Vector|VectorGetAbs (Math|Vector|RotateVectorAroundAxis (.Scale (Math|Transform|BreakTransform _array_element)) (LocalVariables|GetChange_angle) "0, 0,1.000000")))))
  (Utilities|Array|RemoveItem Array_for_delete Door_in)
  (Utilities|Array|RemoveItem Array_for_delete Door_out)
  (Development|PrintString (Utilities|String|Append "Комната Номер: " (Utilities|String|ToString(Integer) (Variables|Default|GetCount_Room))) true true "(R=0.000000,G=0.128517,B=1.000000,A=1.000000)" 3e+01)
  (while (LocalVariables|GetCant_Build)
    (bind _array_element_2 (Utilities|Array|ForEachLoopwithBreak (Variables|/Game/Blueprints/ProcGen/Constructor_Dungeon.Constructor_Dungeon_C|GetSize_Box_Room New_Room) :!label _label)
      (:LoopBody
        (bind (_outcomponents _returnvalue_4) (Collision|BoxOverlapComponents (.Location (Math|Transform|BreakTransform _array_element_2)) (Math|Vector|MakeVector (/ (.x (.Scale (Math|Transform|BreakTransform _array_element_2))) 2.0) (/ (.y (.Scale (Math|Transform|BreakTransform _array_element_2))) 2.0) (/ (.z (.Scale (Math|Transform|BreakTransform _array_element_2))) 2.0)) (Utilities|Array|MakeArray "ObjectTypeQuery2") "/Script/Engine.StaticMeshComponent" (Utilities|Array|MakeArray New_Room) :!class /Script/Engine.KismetSystemLibrary))
        (Development|PrintString (Utilities|String|ToString(Boolean) _returnvalue_4) true true "(R=1.000000,G=0.000000,B=0.091393,A=1.000000)" 3e+01)
        (if _returnvalue_4
          (Development|PrintString (Utilities|String|Append (Utilities|String|ToString(Integer) (Utilities|Array|Length _outcomponents)) "  Вот столько") true true "(R=0.000000,G=0.660000,B=1.000000,A=1.000000)" 1e+02)
          (for _array_element_3 _outcomponents
            (Transformation|SetWorldLocation _array_element_3 (Math|Vector|MakeVector (.x (Transformation|GetWorldLocation _array_element_3)) (.y (Transformation|GetWorldLocation _array_element_3)) 1.5e+02) false false)
            (Development|PrintString (Utilities|GetDisplayName _array_element_3) true true "(R=0.391003,G=1.000000,B=0.869596,A=1.000000)" 1e+02))
          (Transformation|SetActorTransform New_Room (Math|Transform|MakeTransform (+ (.location _returnvalue) (LocalVariables|GetDirection_Step_Change_location)) (.rotation _returnvalue) (.scale _returnvalue)))
          (for (_array_element_4 _array_index_2) (Variables|/Game/Blueprints/ProcGen/Constructor_Dungeon.Constructor_Dungeon_C|GetSize_Box_Room New_Room)
            (Utilities|Array|SetArrayElem (Variables|/Game/Blueprints/ProcGen/Constructor_Dungeon.Constructor_Dungeon_C|GetSize_Box_Room New_Room) _array_index_2 (Math|Transform|MakeTransform (+ (.Location (Math|Transform|BreakTransform _array_element_4)) (LocalVariables|GetDirection_Step_Change_location)) (.Rotation (Math|Transform|BreakTransform _array_element_4)) (.Scale (Math|Transform|BreakTransform _array_element_4))))
            (LocalVariables|SetCant_Build true))
          (goto _label Break)
          (else
            (Development|PrintString "Нет столкновений" true true "(R=0.000000,G=0.660000,B=1.000000,A=1.000000)" 3e+01)
            (LocalVariables|SetCant_Build false))))))
  (Development|PrintString "no" true true "(R=0.000000,G=0.660000,B=1.000000,A=1.000000)" 1e+02)
  (return))