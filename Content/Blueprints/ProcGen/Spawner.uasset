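; Spawner is a test Blueprint, apparently for procedural generation, that spawns actors and probes the world for overlaps.
; BeginPlay spawns two instances of the same class at fixed locations and stores both references.
; Each Tick nudges a query point along X, runs a WorldStatic box overlap there, and prints Russian debug messages with any overlapped actor names.
; A component-overlap query and a second print branch are left unconnected.
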(event EventBeginPlay
  (bind _returnvalue (Game|SpawnActorfromClass "/Game/Blueprints/ProcGen/Actor_.Actor__C" (Math|Transform|MakeTransform "0, 0, 0") "Undefined" 0 0))
  (Variables|Default|SetOne_war _returnvalue)
  (bind _returnvalue_2 (Game|SpawnActorfromClass "/Game/Blueprints/ProcGen/Actor_.Actor__C" (Math|Transform|MakeTransform "100.000000,200.000000,0.000000" "0, 0, 0" "1,1,1.000000") "AlwaysSpawn" 0 0))
  (Variables|Default|Settwo_war _returnvalue_2))

(event EventTick
  (params (DeltaSeconds :type Float%20%28single-precision%29))
  (bind _output_get (Variables|Default|SetNewVar_0 (+ (Variables|Default|GetNewVar_0) "1.000000,0,0")))
  (bind (_outactors _returnvalue) (Collision|BoxOverlapActors _output_get "0, 0, 0" (Utilities|Array|MakeArray "ObjectTypeQuery1") 0 :!class /Script/Engine.KismetSystemLibrary))
  (if _returnvalue
    (Development|PrintString "Есть пересечения" true true "(R=1.000000,G=0.000000,B=0.015913,A=1.000000)" 1.0)
    (for _array_element _outactors
      (Development|PrintString (Utilities|GetDisplayName _array_element) true true "(R=1.000000,G=0.000000,B=0.015913,A=1.000000)" 1.0))
    (else
      (Development|PrintString "Нет пересечений" true true "(R=0.069388,G=1.000000,B=0.000000,A=1.000000)" 1.0))))

(fn ConstructionScript)