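; Wolf enemy character Blueprint that handles the animal's attack, pain and death reactions.
; Attack measures distance to the player and plays a leap montage at or beyond the ranged threshold set on BeginPlay, otherwise a standard attack montage.
; Damage halts walking during a pain montage, then restores speed after a short delay.
; Death reuses the pain montage, then destroys the actor after a delay.
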(event EventBeginPlay
  (Variables|Default|SetDistance_Melee_Attack 1.2e+02)
  (Variables|Default|SetDistance_Range_Attack 2e+02))

(event EventAttack
  (if (>= (Math|Vector|Distance(Vector) (Transformation|GetWorldLocation (Variables|Default|GetCapsuleComponent)) (Transformation|GetWorldLocation (Variables|/Script/Engine.Actor|GetRootComponent (Variables|Default|GetPlayer_Reference)))) (Variables|Default|GetDistance_Range_Attack))
    (Animation|PlayAnimMontage "/Game/Enemies_and_Other_NPC/Wolf/Animation/Wolf_ataka_prijok__Montage.Wolf_ataka_prijok__Montage" 1.0 "None")
    (else
      (Animation|PlayAnimMontage "/Game/Enemies_and_Other_NPC/Wolf/Animation/Wolf_ataka1_Montage.Wolf_ataka1_Montage" 1.0 "None"))))

(event EventBeginAnimationPerDamage
  (Variables|/Script/Engine.CharacterMovementComponent|SetMaxWalkSpeed (Variables|Character|GetCharacterMovement) 0.0)
  (Animation|PlayAnimMontage "/Game/Enemies_and_Other_NPC/Wolf/Animation/Wolf_pain_Montage.Wolf_pain_Montage" 1.0 "None")
  (Utilities|FlowControl|Delay 1.0)
  (Variables|/Script/Engine.CharacterMovementComponent|SetMaxWalkSpeed (Variables|Character|GetCharacterMovement) 5e+02))

(event EventDead
  (Animation|PlayAnimMontage "/Game/Enemies_and_Other_NPC/Wolf/Animation/Wolf_pain_Montage.Wolf_pain_Montage" 1.0 "None")
  (Utilities|FlowControl|Delay 2.0)
  (Actor|DestroyActor))

(fn ConstructionScript)